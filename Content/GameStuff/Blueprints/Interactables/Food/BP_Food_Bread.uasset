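; BP_Food_Bread is a bread food Blueprint whose status changes once over time.
; On BeginPlay it runs the parent logic, then waits for the TimeToStatusChange delay stored in its FoodInfo struct.
; ChangeStatus then sets FoodStatus to one fixed enum value, with debug prints showing the status before and after the change.
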(event EventBeginPlay
  (bind _foodinfo (Variables|Default|GetFoodInfo))
  (bind (_modifyamount _foodstatus _timetostatuschange) (Utilities|Struct|BreakF_FoodInfo _foodinfo))
  (|CallParentFunction)
  (Development|PrintString (Utilities|String|EnumtoString _foodstatus))
  (Utilities|FlowControl|Delay _timetostatuschange)
  (CallFunction|ChangeStatus)
  (Development|PrintString "Status Changed")
  (Development|PrintString (Utilities|String|EnumtoString (.foodstatus (Variables|Default|GetFoodInfo)))))

(fn ConstructionScript
  (|CallParentFunction))

(fn ChangeStatus
  (bind _structout (Utilities|Struct|SetmembersinF_FoodInfo (Variables|Default|GetFoodInfo) "NewEnumerator4"))
  (Variables|Default|SetFoodInfo _structout))
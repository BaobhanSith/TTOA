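; Base interactable item actor that the player can pick up into their inventory.
; The construction script reads the item's data table row to fill ItemInfo and set the interaction mesh.
; Interaction passes the item to the player's PickupMessage.
; AddItem adds the amount by item class to the player's inventory; on success it keeps any remainder in the actor, otherwise destroys it when none remains.
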(event EventBeginPlay)

(event EventInteraction
  (params (Player :type CH%20Player%20Character%20Object%20Reference))
  (Class|BPIInteract|Pickup(Message) Player self))

(fn ConstructionScript
  (bind _item (Variables|Default|GetItem))
  (bind (_datatable _rowname) (Utilities|Struct|BreakDataTableRowHandle _item))
  (bind _returnvalue (Utilities|GetDataTableRow _datatable _rowname)
    (:then
      (Utilities|Struct|SetmembersinF_ItemInfo (Variables|Default|GetItemInfo) (.ItemInternalName (Utilities|Struct|BreakF_ItemInfo _returnvalue)) (.ItemType (Utilities|Struct|BreakF_ItemInfo _returnvalue)) (.ItemRarity (Utilities|Struct|BreakF_ItemInfo _returnvalue)) (.ItemName (Utilities|Struct|BreakF_ItemInfo _returnvalue)) (.ItemDescription (Utilities|Struct|BreakF_ItemInfo _returnvalue)) (.ItemImage (Utilities|Struct|BreakF_ItemInfo _returnvalue)) (.ItemClass (Utilities|Struct|BreakF_ItemInfo _returnvalue)) (.ItemIndex (Utilities|Struct|BreakF_ItemInfo _returnvalue)) (.ItemSlot (Utilities|Struct|BreakF_ItemInfo _returnvalue)) (.ItemValue (Utilities|Struct|BreakF_ItemInfo _returnvalue)) (.ItemWeight (Utilities|Struct|BreakF_ItemInfo _returnvalue)) (.ItemStat (Utilities|Struct|BreakF_ItemInfo _returnvalue)) (.CanBeStacked? (Utilities|Struct|BreakF_ItemInfo _returnvalue)) (.IsQuestItem? (Utilities|Struct|BreakF_ItemInfo _returnvalue)) (.ItemMesh (Utilities|Struct|BreakF_ItemInfo _returnvalue)))
      (Components|StaticMesh|SetStaticMesh (Variables|Default|GetInteractionMesh) (.ItemMesh (Utilities|Struct|BreakF_ItemInfo _returnvalue))))))

(fn AddItem
  (params (Player :type CH%20Player%20Character%20Object%20Reference))
  (bind (_rest _success_) (Default|AddtoInventory Player (Utilities|GetClass self) (Variables|Default|GetAmountToAdd)))
  (if _success_
    (if (> _rest 0)
      (Variables|Default|SetAmountToAdd _rest)
      (else
        (Actor|DestroyActor)))))